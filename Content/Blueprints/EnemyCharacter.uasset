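; Enemy character that takes damage, shows a floating health bar and is destroyed when its health runs out.
; InflictDamage subtracts from Health, then either calls Die, which prints a message and destroys the actor, or refreshes the bar.
; The bar's fill comes from Health relative to the max enemy health stored in MyGameInstance.
; Each Tick rotates the bar's widget component to face the player camera.
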(event `self.ReceiveBeginPlay`
  (`self.SetHealthBarPercentage`))

(event `self.ReceiveTick`
  (params (DeltaSeconds :type "Float (single-precision)"))
  (`self.RotateHealthbarToPlayer`))

(fn `Die`
  (`KismetSystemLibrary.PrintString` "I am dead!")
  (`self.K2_DestroyActor`))

(fn `InflictDamage`
  (params (damage :type "Float (double-precision)"))
  (returns (Output_Get :type "Float (double-precision)"))
  (bind _output_get (set `self.Health` (- (`self.Health`) damage)))
  (if (<= _output_get 0.0)
    (`self.Die`)
    (else
      (`self.SetHealthBarPercentage`)))
  (return (`self.Health`)))

(fn `RotateHealthbarToPlayer`
  (bind _returnvalue (`GameplayStatics.GetPlayerCameraManager` 0))
  (`/Engine/EditorBlueprintResources/StandardMacros.IsValid` _returnvalue
    (:`Is Valid`
      (`SceneComponent.K2_SetWorldRotation` (`self.HealthBar`) (`KismetMathLibrary.FindLookAtRotation` (`SceneComponent.K2_GetComponentLocation` (`self.HealthBar`)) (`PlayerCameraManager.GetCameraLocation` _returnvalue)) false false)
      (return))))

(fn `SetHealthBarPercentage`
  (bind _asmy_game_instance (cast `/Game/Blueprints/MyGameInstance` (`GameplayStatics.GetGameInstance`)))
  (bind _returnvalue (`/Game/Blueprints/MyGameInstance.getEnemyMaxHealth` _asmy_game_instance))
  (bind _asenemy_health_bar (cast `/Game/UI/EnemyHealthBar` (`WidgetComponent.GetUserWidgetObject` (`self.HealthBar`))))
  (`ProgressBar.SetPercent` (`/Game/UI/EnemyHealthBar.ProgressBar_111` _asenemy_health_bar) (* (/ 1.0 _returnvalue) (`self.Health`)))
  (return))

(fn `UserConstructionScript`)