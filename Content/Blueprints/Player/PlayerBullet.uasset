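; PlayerBullet is the player's projectile, which damages enemies it overlaps.
; The construction script sets the ProjectileMovement initial and max speed from a single ProjectileSpeed variable.
; On overlapping an EnemyCharacter it inflicts damage computed from the GameInstance's base projectile damage and multiplier, then destroys itself.
; It ignores overlaps with FirstPersonCharacter and destroys itself on contact with any other actor.
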(event `self.ReceiveActorBeginOverlap`
  (params (OtherActor :type "Actor Object Reference"))
  (bind _asenemy_character (cast `/Game/Blueprints/Enemy/EnemyCharacter` OtherActor)
    (:`then`
      (bind _returnvalue (`self.GetBulletDamage`))
      (`/Game/Blueprints/Enemy/EnemyCharacter.InflictDamage` _asenemy_character _returnvalue)
      (`self.K2_DestroyActor`))
    (:`CastFailed`
      (cast `/Game/Blueprints/Player/FirstPersonCharacter` OtherActor
        (:`CastFailed`
          (`self.K2_DestroyActor`))))))

(fn `GetBulletDamage`
  (returns (ReturnValue :type "Float (double-precision)"))
  (bind _asmy_game_instance (cast `/Game/Blueprints/MyGameInstance` (`GameplayStatics.GetGameInstance`)))
  (return (* (`/Game/Blueprints/MyGameInstance.PlayerProjectileDamage` _asmy_game_instance) (`/Game/Blueprints/MyGameInstance.PlayerProjectileDamageMultiplier` _asmy_game_instance))))

(fn `UserConstructionScript`
  (bind _projectilemovement (`self.ProjectileMovement`))
  (bind _output_get (set `ProjectileMovementComponent.MaxSpeed` (`self.ProjectileSpeed`) _projectilemovement))
  (set `ProjectileMovementComponent.InitialSpeed` _output_get _projectilemovement))