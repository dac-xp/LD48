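; Enemy character that fires projectiles at the player, shows a health bar that turns to face the camera, and is destroyed when its health runs out.
; Max health, capsule scale and projectile speed come from MyGameInstance.
; StartShooting and StopShooting toggle firing; Tick spawns EnemyBullets aimed from the muzzle while the player lives, with a short Delay as cooldown.
; InflictDamage updates the health bar widget or calls Die.
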(event `self.ReceiveBeginPlay`
  (bind _asmy_game_instance (cast `/Game/Blueprints/MyGameInstance` (`GameplayStatics.GetGameInstance`)))
  (bind _returnvalue (`/Game/Blueprints/MyGameInstance.getEnemyMaxHealth` _asmy_game_instance))
  (set `self.Health` _returnvalue)
  (`self.SetHealthBarPercentage`)
  (`SceneComponent.SetWorldScale3D` (`self.CapsuleComponent`) (`KismetMathLibrary.Conv_DoubleToVector` (`/Game/Blueprints/MyGameInstance.EnemySizeMultiplicator` _asmy_game_instance))))

(event `self.ReceiveTick`
  (params (DeltaSeconds :type "Float (single-precision)"))
  (`self.RotateHealthbarToPlayer`)
  (bind _asmy_game_instance (cast `/Game/Blueprints/MyGameInstance` (`GameplayStatics.GetGameInstance`)))
  (bind _asfirst_person_character (cast `/Game/Blueprints/Player/FirstPersonCharacter` (`GameplayStatics.GetPlayerCharacter` 0)))
  (if (and (> (`/Game/Blueprints/MyGameInstance.PlayerHealth` _asmy_game_instance) 0.0) (not (`/Game/Blueprints/Player/FirstPersonCharacter.IsDead` _asfirst_person_character)))
    (bind _didshoot1 (`self.Shoot`))
    (if _didshoot1
      (`KismetSystemLibrary.Delay` 0.5)
      (set `self.isAllowedToShoot` true))))

(event `StartShooting`
  (set `self.isShooting` true))

(event `StopShooting`
  (set `self.isShooting` false))

(fn `Die`
  (`KismetSystemLibrary.PrintString` "I am dead!")
  (`self.K2_DestroyActor`))

(fn `InflictDamage`
  (params (damage :type "Float (double-precision)"))
  (returns (Output_Get :type "Float (double-precision)"))
  (bind _output_get (set `self.Health` (- (`self.Health`) damage)))
  (if (<= _output_get 0.0)
    (`self.Die`)
    (else
      (`self.SetHealthBarPercentage`)))
  (return (`self.Health`)))

(fn `RotateHealthbarToPlayer`
  (bind _returnvalue (`GameplayStatics.GetPlayerCameraManager` 0))
  (`/Engine/EditorBlueprintResources/StandardMacros.IsValid` _returnvalue
    (:`Is Valid`
      (`SceneComponent.K2_SetWorldRotation` (`self.HealthBar`) (`KismetMathLibrary.FindLookAtRotation` (`SceneComponent.K2_GetComponentLocation` (`self.HealthBar`)) (`PlayerCameraManager.GetCameraLocation` _returnvalue)) false false)
      (return))))

(fn `SetHealthBarPercentage`
  (bind _asmy_game_instance (cast `/Game/Blueprints/MyGameInstance` (`GameplayStatics.GetGameInstance`)))
  (bind _returnvalue (`/Game/Blueprints/MyGameInstance.getEnemyMaxHealth` _asmy_game_instance))
  (bind _asenemy_health_bar (cast `/Game/UI/EnemyHealthBar` (`WidgetComponent.GetUserWidgetObject` (`self.HealthBar`))))
  (`ProgressBar.SetPercent` (`/Game/UI/EnemyHealthBar.ProgressBar_111` _asenemy_health_bar) (* (/ 1.0 _returnvalue) (`self.Health`)))
  (return))

(fn `Shoot`
  (returns (didShoot1 :type Boolean))
  (locals (didShoot :type Boolean))
  (bind _returnvalue (`SceneComponent.K2_GetComponentLocation` (`self.Muzzle`)))
  (if (and (`self.isAllowedToShoot`) (`self.isShooting`))
    (set `local.didShoot` true)
    (bind _asmy_game_instance (cast `/Game/Blueprints/MyGameInstance` (`GameplayStatics.GetGameInstance`)))
    (`|SpawnActorFromClass` "/Game/Blueprints/Enemy/EnemyBullet.EnemyBullet_C" (`KismetMathLibrary.MakeTransform` _returnvalue (`KismetMathLibrary.FindLookAtRotation` _returnvalue (+ (`SceneComponent.K2_GetComponentLocation` (`Actor.RootComponent` (`GameplayStatics.GetPlayerCharacter` 0))) (0.0 5.0 0.0)))) "Undefined" "OverrideRootScale" null (* (`/Game/Blueprints/MyGameInstance.EnemyProjectileSpeed` _asmy_game_instance) (`/Game/Blueprints/MyGameInstance.EnemyProjectileSpeedMultiplicator` _asmy_game_instance)) null)
    (set `self.isAllowedToShoot` false)
    (else
      (set `local.didShoot` false)))
  (return (`local.didShoot`)))

(fn `UserConstructionScript`)