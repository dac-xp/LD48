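; EnemyBullet is an enemy projectile that damages the first-person player on overlap.
; The construction script sets both the initial and max speed of its projectile movement from the ProjectileSpeed variable.
; On overlapping the player character, it reads the enemy damage value from MyGameInstance, calls InflictDamage on the player, then destroys itself.
; Overlapping any other actor simply destroys it.
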(event `self.ReceiveActorBeginOverlap`
  (params (OtherActor :type "Actor Object Reference"))
  (bind _asfirst_person_character (cast `/Game/Blueprints/Player/FirstPersonCharacter` OtherActor)
    (:`then`
      (bind _asmy_game_instance (cast `/Game/Blueprints/MyGameInstance` (`GameplayStatics.GetGameInstance`)))
      (bind _returnvalue (`/Game/Blueprints/MyGameInstance.getEnemyDamage` _asmy_game_instance))
      (`/Game/Blueprints/Player/FirstPersonCharacter.inflictDamage` _asfirst_person_character _returnvalue)
      (`self.K2_DestroyActor`))
    (:`CastFailed`
      (`self.K2_DestroyActor`))))

(fn `UserConstructionScript`
  (bind _projectilemovement (`self.ProjectileMovement`))
  (bind _output_get (set `ProjectileMovementComponent.MaxSpeed` (`self.ProjectileSpeed`) _projectilemovement))
  (set `ProjectileMovementComponent.InitialSpeed` _output_get _projectilemovement))