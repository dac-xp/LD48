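; Game instance that holds level progression and enemy scaling stats across map reloads.
; Getter functions return enemy max health and damage as base values times their multipliers.
; LoadNextLevel increments the level counter, raises the enemy size and damage multipliers, then reopens the same first-person example map.
; The health multiplier is not changed in these graphs.
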(fn `getEnemyDamage`
  (returns (ReturnValue :type "Float (double-precision)"))
  (return (* (`self.EnemyDamage`) (`self.EnemyDamageMultiplier`))))

(fn `getEnemyMaxHealth`
  (returns (ReturnValue :type "Float (double-precision)"))
  (return (* (`self.EnemyMaxHealth`) (`self.EnemyMaxHealthMultiplier`))))

(fn `LoadNextLevel`
  (set `self.CurrentLevel` (+ (`self.CurrentLevel`) 1))
  (set `self.EnemySizeMultiplicator` (+ (`self.EnemySizeMultiplicator`) 0.1))
  (set `self.EnemyDamageMultiplier` (+ (`self.EnemyDamageMultiplier`) 0.1))
  (`GameplayStatics.OpenLevel` "FirstPersonExampleMap"))