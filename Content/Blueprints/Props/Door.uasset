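; Level exit door that opens only once no actors tagged Enemy remain, and ends the level when the player overlaps it.
; Interact plays an Actor Sequence to open the door once, or prints a message while enemies remain.
; Player overlap gets a generated mutation from MyGameInstance and passes it to the character's end-of-level HUD, without checking whether the door is open.
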(event `/Game/Blueprints/Interactable.Interact`
  (bind _outactors (`GameplayStatics.GetAllActorsWithTag` "Enemy"))
  (if (== (`KismetArrayLibrary.Array_Length` _outactors) 0)
    (if (not (`self.isOpen`))
      (`MovieSceneSequencePlayer.Play` (`ActorSequenceComponent.SequencePlayer` (`self.ActorSequence`)))
      (set `self.isOpen` true))
    (else
      (`KismetSystemLibrary.PrintString` "There are still enemies here"))))

(event `self.ReceiveActorBeginOverlap`
  (params (OtherActor :type "Actor Object Reference"))
  (if (`self.ActorHasTag` OtherActor "Player")
    (bind _asfirst_person_character (cast `/Game/Blueprints/Player/FirstPersonCharacter` (`GameplayStatics.GetPlayerCharacter` 0)))
    (bind _asmy_game_instance (cast `/Game/Blueprints/MyGameInstance` (`GameplayStatics.GetGameInstance`)))
    (bind _returnvalue (`/Game/Blueprints/MyGameInstance.GeneratePlayerMutation` _asmy_game_instance))
    (`/Game/Blueprints/Player/FirstPersonCharacter.ShowEndOfLevelHUD` _asfirst_person_character _returnvalue)))

(fn `UserConstructionScript`)